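; BP_TestGameMode is a test game mode holding logic to spawn a square grid of BP_InefficientActor instances.
; Nested loops over TotalRowsCols place actors Spacing units apart at Z zero, offset by half the grid size to roughly center it on the world origin.
; The spawn loop is disconnected and never runs, as BeginPlay and the construction script are both empty.
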(event `self.ReceiveBeginPlay`)

(fn `UserConstructionScript`)